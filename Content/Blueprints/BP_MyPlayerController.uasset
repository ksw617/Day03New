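; Player controller that routes input to the possessed BP_Character for movement, jumping and attacking.
; On BeginPlay it casts player pawn 0 to BP_Character and caches the reference.
; Axis inputs move the character along its actor forward and right vectors, Jump calls the character's jump, and Attack plays the AM_Attack montage directly.
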(event `self.ReceiveBeginPlay`
  (bind _asbp_character (cast `/Game/Blueprints/BP_Character` (`GameplayStatics.GetPlayerPawn` 0)))
  (set `self.MyCharacter` _asbp_character))

(event `InputAxis|MoveForwardBackward`
  (params (AxisValue :type "Float (single-precision)"))
  (`Pawn.AddMovementInput` (`self.MyCharacter`) (`self.GetActorForwardVector` (`self.MyCharacter`)) AxisValue false))

(event `InputAxis|MoveLeftRight`
  (params (AxisValue :type "Float (single-precision)"))
  (`Pawn.AddMovementInput` (`self.MyCharacter`) (`self.GetActorRightVector` (`self.MyCharacter`)) AxisValue false))

(event `InputAction|Attack`
  (params (Key :type "Key Structure"))
  (:`Pressed`
    (`Character.PlayAnimMontage` (`self.MyCharacter`) "/Game/Animations/AM_Attack.AM_Attack" 1.0 "None")))

(event `InputAction|Jump`
  (params (Key :type "Key Structure"))
  (:`Pressed`
    (`Character.Jump` (`self.MyCharacter`))))

(fn `UserConstructionScript`)